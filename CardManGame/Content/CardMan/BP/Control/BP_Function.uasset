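; BP_Function is a set of helper functions for reading and writing the local player's state and action state.
; Each getter and setter fetches player controller 0, takes its PlayerState and forwards to the matching FGet or FSet message call on it.
; The message calls appear to go through an interface, so no cast to a specific PlayerState class is needed.
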(fn `F2_GetSelfPlayerActionState`
  (returns (PlayerActionState :type "/Game/CardMan/BP/Enumerate/E_PlayerActionState Enum"))
  (bind _playeractionstate (message `/Game/CardMan/BP/Control/IN_PlayerStateInterface.F_GetPlayerActionState` (`Controller.PlayerState` (`GameplayStatics.GetPlayerController` null))))
  (return _playeractionstate))

(fn `F2_GetSelfPlayerState`
  (returns (PlayerState :type "/Game/CardMan/BP/Enumerate/ST_PlayerState Structure"))
  (bind _playerstate (message `/Game/CardMan/BP/Control/IN_PlayerStateInterface.F_GetPlayerState` (`Controller.PlayerState` (`GameplayStatics.GetPlayerController` null))))
  (return _playerstate))

(fn `F2_SetSelfPlayerActionState`
  (params (NewParam :type "/Game/CardMan/BP/Enumerate/E_PlayerActionState Enum" :default "NewEnumerator0"))
  (message `/Game/CardMan/BP/Control/IN_PlayerStateInterface.F_SetPlayerActionState` (`Controller.PlayerState` (`GameplayStatics.GetPlayerController` null)) NewParam)
  (return))

(fn `F2_SetSelfPlayerState`
  (params (PlayerState :type "/Game/CardMan/BP/Enumerate/ST_PlayerState Structure"))
  (message `/Game/CardMan/BP/Control/IN_PlayerStateInterface.F_SetPlayerState` (`Controller.PlayerState` (`GameplayStatics.GetPlayerController` null)) PlayerState)
  (return))