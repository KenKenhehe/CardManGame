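; Player controller for the CardMan character that handles camera setup, combat input and damage lookup.
; On BeginPlay it spawns and views through a BP_Camera, then binds the anim blueprint's SpawnThrow dispatcher to spawn BP_ThrowObject through a server event.
; Mouse and Space keys message the anim instance for attack, dodge and energy-gated magic throw montages.
; GetHowMuchDamage detects backstabs by yaw but only prints them, returning the player state's Attack unchanged.
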(event `self.ReceiveBeginPlay`
  (bind _returnvalue (`GameplayStatics.GetPlayerPawn` 0))
  (bind _asbp_character (cast `/Game/CardMan/BP/Character/BP_Character` _returnvalue))
  (set `self.BP_Character` _asbp_character)
  (bind _returnvalue_2 (`|SpawnActorFromClass` "/Game/CardMan/BP/Character/BP_Camera.BP_Camera_C" (`self.GetTransform` _returnvalue) "Undefined" "OverrideRootScale" null _returnvalue null))
  (`self.SetViewTargetWithBlend` _returnvalue_2)
  (`WidgetBlueprintLibrary.SetInputMode_GameAndUIEx` self null)
  (bind _asabp_character_animation (cast `/Game/CardMan/BP/Character/ABP_CharacterAnimation` (`SkeletalMeshComponent.GetAnimInstance` (`Character.Mesh` (`self.BP_Character`)))))
  (add `/Game/CardMan/BP/Character/ABP_CharacterAnimation.SpawnThrow` _asabp_character_animation (delegate `SpawnThrow_Event_0`)))

(event `SpawnThrow_Event_0`
  (`self.Event_Server_SpawnThrow`))

(event `Event_Server_SpawnThrow`
  (bind _bp_character (`self.BP_Character`))
  (`|SpawnActorFromClass` "/Game/CardMan/BP/Items/BP_ThrowObject.BP_ThrowObject_C" (`KismetMathLibrary.MakeTransform` (.location (`self.GetTransform` _bp_character)) (.rotation (`self.GetTransform` _bp_character))) "Undefined" "OverrideRootScale" null (`self.GetActorForwardVector` _bp_character) null))

(event `Key|LeftMouseButton`
  (params (Key :type "Key Structure"))
  (:`Pressed`
    (message `/Game/CardMan/BP/Control/IN_PlayerAnimInterface.F_PlayerAttackMontage` (`SkeletalMeshComponent.GetAnimInstance` (`Character.Mesh` (`self.BP_Character`))))))

(event `Key|SpaceBar`
  (params (Key :type "Key Structure"))
  (:`Pressed`
    (message `/Game/CardMan/BP/Control/IN_PlayerAnimInterface.F_PlayerDodgeMontage` (`SkeletalMeshComponent.GetAnimInstance` (`Character.Mesh` (`self.BP_Character`))))))

(event `Key|RightMouseButton`
  (params (Key :type "Key Structure"))
  (:`Pressed`
    (if (>= (`.CurrentEnergyCount_13_0C45F6AB41D1F0F6FAC95FBBD7F3C080` (break `/Game/CardMan/BP/Enumerate/ST_PlayerState` (`/Game/CardMan/BP/Control/BP_Function.F2_GetSelfPlayerState`))) 1)
      (message `/Game/CardMan/BP/Control/IN_PlayerAnimInterface.F_PlayerMagicThrowMontage` (`SkeletalMeshComponent.GetAnimInstance` (`Character.Mesh` (`self.BP_Character`)))))))

(fn `GetHowMuchDamage`
  (params (Enemy :type "Actor Object Reference"))
  (returns (Damage :type "Float (double-precision)"))
  (locals (BackAttack :type Boolean))
  (bind _yaw (.yaw (`KismetMathLibrary.NormalizedDeltaRotator` (`KismetMathLibrary.FindLookAtRotation` (`self.K2_GetActorLocation` (`self.BP_Character`)) (`self.K2_GetActorLocation` Enemy)) (`self.K2_GetActorRotation` Enemy))))
  (bind _output_get (set `local.BackAttack` (and (> _yaw -90.0) (< _yaw 90.0))))
  (`KismetSystemLibrary.PrintString` (select `bool` _output_get :`true` "被刺"))
  (bind _playerstate (message `/Game/CardMan/BP/Control/IN_PlayerStateInterface.F_GetPlayerState` (`self.PlayerState`)))
  (return (`.Attack_10_01A2860D4B3B967C429F40A169956EC2` (break `/Game/CardMan/BP/Enumerate/ST_PlayerState` _playerstate))))

(fn `UserConstructionScript`)