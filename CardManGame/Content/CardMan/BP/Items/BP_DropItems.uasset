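; BP_DropItems is a dropped-item actor that pops out when spawned and disappears on overlap.
; On BeginPlay it picks a random mesh from StaticMeshRandom and throws its Box with a random sideways and upward impulse.
; The Item timeline then animates the mesh's relative height and rotation for a float-and-spin effect.
; Any overlap beginning on the Box destroys the actor, with no filter or reward logic.
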(event `self.ReceiveBeginPlay`
  (bind _returnvalue (`KismetMathLibrary.RandomFloatInRange` -20000.0 20000.0))
  (bind _staticmesh_random (`self.staticMesh_Random`))
  (bind _staticmesh (`self.StaticMesh`))
  (`StaticMeshComponent.SetStaticMesh` _staticmesh (`|GetArrayItem` _staticmesh_random (`KismetMathLibrary.RandomIntegerInRange` 0 (- (`KismetArrayLibrary.Array_Length` _staticmesh_random) 1))))
  (`PrimitiveComponent.AddImpulseAtLocation` (`self.Box`) (`KismetMathLibrary.MakeVector` _returnvalue _returnvalue (`KismetMathLibrary.RandomFloatInRange` 30000.0 50000.0)) (`self.K2_GetActorLocation`) "None")
  (bind (_direction _rotation _location) (`Timeline|Item`)
    (:`Update`
      (`SceneComponent.K2_SetRelativeLocationAndRotation` _staticmesh (`KismetMathLibrary.VLerp` (0.0 0.0 0.0) (0.0 0.0 100.0) _location) (`KismetMathLibrary.RLerp` (struct) (struct :`Yaw` 360.0) _rotation) false false))))

(event `self.Box.OnComponentBeginOverlap`
  (params (OverlappedComponent :type "PrimitiveComponent Object Reference") (OtherActor :type "Actor Object Reference") (OtherComp :type "PrimitiveComponent Object Reference") (OtherBodyIndex :type Integer) (bFromSweep :type Boolean) (SweepResult :type "HitResult Structure (by ref)"))
  (`self.K2_DestroyActor`))

(fn `UserConstructionScript`)