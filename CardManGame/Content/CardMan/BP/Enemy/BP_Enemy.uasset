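; Enemy actor that takes damage, collects attached throw-object nodes and scatters drops when it dies.
; AnyDamage lowers HP in its state struct; at zero it releases held nodes as BP_ThrowObjectNode, destroys itself and spawns random BP_DropItems.
; AddObject raises the energy count and attaches a BP_ThrowObjectNode_Enemy to the capsule, tracked in the Tag array.
; When a node's delay-over dispatcher fires, it is replaced by a BP_ThrowObjectNode randomly placed nearby.
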(event `self.ReceiveAnyDamage`
  (params (Damage :type "Float (single-precision)") (DamageType :type "DamageType Object Reference") (InstigatedBy :type "Controller Object Reference") (DamageCauser :type "Actor Object Reference"))
  (bind _returnvalue (`KismetMathLibrary.RandomFloatInRange` 0.0 50.0))
  (bind _enemystate (`self.EnemyState`))
  (`KismetSystemLibrary.PrintString` (`KismetStringLibrary.Conv_DoubleToString` Damage))
  (bind _structout (setmembers `/Game/CardMan/BP/Enumerate/ST_PlayerState` :`StructRef` _enemystate :`CurrentHP` (- (`.CurrentHP_8_14464AAC4C6C6F1ACD64B0B9CC427607` (break `/Game/CardMan/BP/Enumerate/ST_PlayerState` _enemystate)) Damage)))
  (if (<= (`.CurrentHP_8_14464AAC4C6C6F1ACD64B0B9CC427607` (break `/Game/CardMan/BP/Enumerate/ST_PlayerState` _structout)) 0.0)
    ;[1 1 1] Enemy Dead
    (setmembers `/Game/CardMan/BP/Enumerate/ST_PlayerState` :`StructRef` (`self.EnemyState`) :`CurrentHP` 0.0)
    (for _array_element (`self.Tag`)
      (`|SpawnActorFromClass` "/Game/CardMan/BP/Items/BP_ThrowObjectNode.BP_ThrowObjectNode_C" (`self.GetTransform`) "Undefined" "OverrideRootScale" null null)
      (`self.K2_DestroyActor` _array_element))
    (`self.K2_DestroyActor`)
    (for _ (range (`KismetMathLibrary.RandomIntegerInRange` 3 5))
      (`|SpawnActorFromClass` "/Game/CardMan/BP/Items/BP_DropItems.BP_DropItems_C" (`KismetMathLibrary.MakeTransform` (`KismetMathLibrary.RandomPointInBoundingBox` (`self.K2_GetActorLocation`) (`KismetMathLibrary.MakeVector` _returnvalue _returnvalue _returnvalue))) "AlwaysSpawn" "OverrideRootScale" null null))))

(event `AddObject`
  (bind _enemystate (`self.EnemyState`))
  (setmembers `/Game/CardMan/BP/Enumerate/ST_PlayerState` :`StructRef` _enemystate :`CurrentEnergyCount` (+ (`.CurrentEnergyCount_13_0C45F6AB41D1F0F6FAC95FBBD7F3C080` (break `/Game/CardMan/BP/Enumerate/ST_PlayerState` _enemystate)) 1))
  ;[1 1 1] Bind Throw Object
  (bind _returnvalue (`|SpawnActorFromClass` "/Game/CardMan/BP/Items/BP_ThrowObjectNode_Enemy.BP_ThrowObjectNode_Enemy_C" (`KismetMathLibrary.MakeTransform` (0.0 0.0 0.0)) "Undefined" "OverrideRootScale" null null))
  (`self.K2_AttachToComponent` _returnvalue (`self.CapsuleComponent`) "None" "KeepRelative" "KeepRelative" "KeepRelative" true)
  (`KismetArrayLibrary.Array_Add` (`self.Tag`) _returnvalue)
  (add `/Game/CardMan/BP/Items/BP_ThrowObjectNode_Enemy.IsDelayOver` _returnvalue (delegate `IsDelayOver_Event`)))

(event `IsDelayOver_Event`
  (params (Tag :type "Actor Object Reference"))
  ;[1 1 1] Bind Throw Object
  (`KismetArrayLibrary.Array_RemoveItem` (`self.Tag`) Tag)
  (`self.K2_DestroyActor` Tag)
  (`|SpawnActorFromClass` "/Game/CardMan/BP/Items/BP_ThrowObjectNode.BP_ThrowObjectNode_C" (`KismetMathLibrary.MakeTransform` (`KismetMathLibrary.MakeVector` (+ (`KismetMathLibrary.RandomFloatInRange` -500.0 500.0) (.x (.location (`self.GetTransform`)))) (+ (.y (.location (`self.GetTransform`))) (`KismetMathLibrary.RandomFloatInRange` -500.0 500.0)) (.z (.location (`self.GetTransform`))))) "Undefined" "OverrideRootScale" null null))

(fn `UserConstructionScript`)